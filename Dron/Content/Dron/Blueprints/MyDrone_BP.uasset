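; Drone Blueprint that sets up the main HUD, projectile class and materials, and shows the win or game-over screen.
; BeginPlay adds the Main_WD widget and assigns the projectile class plus main, shield and damage materials.
; GameWinF and GameOverF each create a shared WinOrDead widget, pick its switcher page and show the mouse cursor.
; No firing, movement or damage logic lives in this graph, and nothing here calls the end-game events.
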(event EventBeginPlay
  (bind _returnvalue (UserInterface|CreateWidget "/Game/Dron/Widget/Main_WD.Main_WD_C"))
  (UserInterface|Viewport|AddtoViewport _returnvalue 0)
  (Variables|Default|SetProjectileClass "/Game/Dron/Blueprints/MyA_Projectile.MyA_Projectile_C")
  (Variables|Default|SetMainMaterial "/Game/Dron/Assets/Drone_Mat.Drone_Mat")
  (Variables|Default|SetShieldMaterial "/Game/Dron/Assets/Shield_Mat.Shield_Mat")
  (Variables|Default|SetDamageMaterial "/Game/Dron/Assets/HP_Mat.HP_Mat"))

(event Collision|EventActorBeginOverlap
  (params (OtherActor :type Actor%20Object%20Reference)))

(event EventTick
  (params (DeltaSeconds :type Float%20%28single-precision%29)))

(event EventGameWinF
  (Development|PrintString "Win")
  (bind _returnvalue (UserInterface|CreateWidget "/Game/Dron/Widget/WinOrDead.WinOrDead_C"))
  (bind _output_get (Variables|Default|SetWinOrDeadWdRef _returnvalue))
  (UserInterface|Viewport|AddtoViewport _output_get 0)
  (Class|WidgetSwitcher|SetActiveWidgetIndex (Variables|/Game/Dron/Widget/WinOrDead.WinOrDead_C|GetWidgetSwitcher_58 _output_get))
  (Variables|/Script/Engine.PlayerController|SetbShowMouseCursor (Game|GetPlayerController 0) true))

(event EventGameOverF
  (Development|PrintString "Dead")
  (bind _returnvalue (UserInterface|CreateWidget "/Game/Dron/Widget/WinOrDead.WinOrDead_C"))
  (bind _output_get (Variables|Default|SetWinOrDeadWdRef _returnvalue))
  (UserInterface|Viewport|AddtoViewport _output_get 0)
  (Class|WidgetSwitcher|SetActiveWidgetIndex (Variables|/Game/Dron/Widget/WinOrDead.WinOrDead_C|GetWidgetSwitcher_58 _output_get) 1)
  (Variables|/Script/Engine.PlayerController|SetbShowMouseCursor (Game|GetPlayerController 0) true))

(fn ConstructionScript)